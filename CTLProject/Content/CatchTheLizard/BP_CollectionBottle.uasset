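; BP_CollectionBottle is the bottle in Catch The Lizard where lizards are deposited.
; On BeginPlay it finds and caches the BP_LizardCollectionManager in the level.
; Each Tick, until the manager flags Victory, it polls DepositVolume for overlapping BP_Lizard actors and passes each one, with itself, to the manager's RecordDeposit.
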(event EventBeginPlay
  (CallFunction|ResolveCollectionManager))

(event Collision|EventActorBeginOverlap
  (params (OtherActor :type Actor%20Object%20Reference)))

(event EventTick
  (params (DeltaSeconds :type Float%20%28single-precision%29))
  (CallFunction|UpdateDeposits))

(fn ConstructionScript)

(fn ResolveCollectionManager
  (bind _returnvalue (Actor|GetActorOfClass "/Game/CatchTheLizard/BP_LizardCollectionManager.BP_LizardCollectionManager_C"))
  (bind _asbp_lizard_collection_manager (Utilities|Casting|CastToBP_LizardCollectionManager _returnvalue))
  (Variables|Default|SetCollectionManager _asbp_lizard_collection_manager)
  (return))

(fn UpdateDeposits
  (if (Utilities|IsValid (Variables|Default|GetCollectionManager))
    (if (not (Variables|/Game/CatchTheLizard/BP_LizardCollectionManager.BP_LizardCollectionManager_C|GetbVictory (Variables|Default|GetCollectionManager)))
      (for _array_element (Collision|GetOverlappingActors (Variables|Default|GetDepositVolume) "/Game/CatchTheLizard/BP_Lizard.BP_Lizard_C" :!class /Script/Engine.PrimitiveComponent)
        (Default|RecordDeposit (Variables|Default|GetCollectionManager) _array_element self))
      (return)
      (else
        (return)))
    (else
      (return))))