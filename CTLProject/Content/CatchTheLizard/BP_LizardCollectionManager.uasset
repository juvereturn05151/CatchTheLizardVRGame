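; Round manager for Catch the Lizard that tracks lizards stored in bottles and triggers victory when all are collected.
; RecordDeposit counts each registered lizard once, only after TryStoreInBottle succeeds.
; Victory locks player and tool input, removes menus, then shows results in a head-facing VR panel or a viewport widget.
; Afterwards, triggers drive both hands' widget clicks once both have been released, and RestartRound reloads the level.
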(event Input|EnhancedActionEvents|EnhancedInputActionIA_Hand_IndexCurl_Left
  (params (ActionValue :type Float%20%28double-precision%29) (ElapsedSeconds :type Float%20%28double-precision%29) (TriggeredSeconds :type Float%20%28double-precision%29) (InputAction :type Input%20Action%20Object%20Reference :default "/Game/XRFramework/Input/Actions/Hands/IA_Hand_IndexCurl_Left.IA_Hand_IndexCurl_Left"))
  (:Triggered
    (Variables|Default|SetLeftTriggerValue ActionValue))
  (:Canceled
    (Variables|Default|SetLeftTriggerValue 0.0))
  (:Completed
    (Variables|Default|SetLeftTriggerValue 0.0)))

(event Input|EnhancedActionEvents|EnhancedInputActionIA_Hand_IndexCurl_Right
  (params (ActionValue :type Float%20%28double-precision%29) (ElapsedSeconds :type Float%20%28double-precision%29) (TriggeredSeconds :type Float%20%28double-precision%29) (InputAction :type Input%20Action%20Object%20Reference :default "/Game/XRFramework/Input/Actions/Hands/IA_Hand_IndexCurl_Right.IA_Hand_IndexCurl_Right"))
  (:Triggered
    (Variables|Default|SetRightTriggerValue ActionValue))
  (:Canceled
    (Variables|Default|SetRightTriggerValue 0.0))
  (:Completed
    (Variables|Default|SetRightTriggerValue 0.0)))

(event EventBeginPlay
  (CallFunction|InitializeCollection))

(event Collision|EventActorBeginOverlap
  (params (OtherActor :type Actor%20Object%20Reference)))

(event EventTick
  (params (DeltaSeconds :type Float%20%28single-precision%29))
  (CallFunction|UpdateVictoryInput))

(fn ConstructionScript)

(fn CompleteVictory
  (bind _returnvalue (Game|GetPlayerController 0))
  (bind _playerpawnref (Variables|Default|GetPlayerPawnRef))
  (if (not (Variables|Default|GetbVictory))
    (if (and (> (Variables|Default|GetTotalLizards) 0) (== (Variables|Default|GetTotalLizards) (Variables|Default|GetStoredLizards)))
      (Variables|Default|SetbVictory true)
      (Variables|Default|SetbVictoryUIArmed false)
      (Variables|/Game/XRFramework/Blueprints/BP_XRPawn.BP_XRPawn_C|SetbCollectionInputLocked _playerpawnref true)
      (Input|DisableInput _playerpawnref _returnvalue)
      (Input|SetIgnoreMoveInput _returnvalue true)
      (Input|SetIgnoreLookInput _returnvalue true)
      (bind _outactors (Actor|GetAllActorsOfClass "/Game/CatchTheLizard/BP_Broom.BP_Broom_C"))
      (for _array_element _outactors
        (Input|DisableInput _array_element _returnvalue)
        (Actor|Tick|SetActorTickEnabled _array_element))
      (bind _outactors_2 (Actor|GetAllActorsOfClass "/Game/CatchTheLizard/BP_Spray.BP_Spray_C"))
      (for _array_element_2 _outactors_2
        (bind _asbp_spray (Utilities|Casting|CastToBP_Spray _array_element_2))
        (Default|UpdateEmission _asbp_spray 0.0 false)
        (Input|DisableInput _array_element_2 _returnvalue)
        (Actor|Tick|SetActorTickEnabled _array_element_2))
      (bind _outactors_3 (Actor|GetAllActorsOfClass "/Game/CatchTheLizard/BP_CollectionBottle.BP_CollectionBottle_C"))
      (for _array_element_3 _outactors_3
        (Input|DisableInput _array_element_3 _returnvalue)
        (Actor|Tick|SetActorTickEnabled _array_element_3))
      (bind _outactors_4 (Actor|GetAllActorsOfClass "/Game/XRFramework/Blueprints/BP_Menu.BP_Menu_C"))
      (for _array_element_4 _outactors_4
        (Actor|DestroyActor _array_element_4))
      (CallFunction|ShowVictory)
      (return)
      (else
        (return)))
    (else
      (return))))

(fn InitializeCollection
  (bind _outactors (Actor|GetAllActorsOfClass "/Game/CatchTheLizard/BP_Lizard.BP_Lizard_C"))
  (Variables|Default|SetRegisteredLizards _outactors)
  (Utilities|Array|Clear (Variables|Default|GetStoredActors))
  (Variables|Default|SetStoredLizards 0)
  (Variables|Default|SetbVictory false)
  (Variables|Default|SetTotalLizards (Utilities|Array|Length (Variables|Default|GetRegisteredLizards)))
  (bind _asbp_xrpawn (Utilities|Casting|CastToBP_XRPawn (Game|Player|GetPlayerPawn 0)))
  (Variables|Default|SetPlayerPawnRef _asbp_xrpawn)
  (Input|EnableInput (Game|GetPlayerController 0))
  (return))

(fn RecordDeposit
  (params (Lizard :type Actor%20Object%20Reference) (Bottle :type BP%20Collection%20Bottle%20Object%20Reference))
  ;[0.15 0.15 0.15 0.5] Unique actor references are the source of truth. Count only after TryStoreInBottle succeeds. Repeated overlaps, attempts, or other bottles cannot increment twice. Zero lizards never produces a premature victory.
  (if (not (Variables|Default|GetbVictory))
    (if (Utilities|Array|ContainsItem (Variables|Default|GetRegisteredLizards) Lizard)
      (if (not (Utilities|Array|ContainsItem (Variables|Default|GetStoredActors) Lizard))
        (bind _asbp_lizard (Utilities|Casting|CastToBP_Lizard Lizard))
        (bind _accepted (Default|TryStoreinBottle _asbp_lizard Bottle))
        (if _accepted
          (Utilities|Array|AddUnique (Variables|Default|GetStoredActors) Lizard)
          (Variables|Default|SetStoredLizards (Utilities|Array|Length (Variables|Default|GetStoredActors)))
          (if (and (> (Variables|Default|GetTotalLizards) 0) (== (Variables|Default|GetStoredLizards) (Variables|Default|GetTotalLizards)))
            (CallFunction|CompleteVictory)
            (return true)
            (else
              (return true)))
          (else
            (return false)))
        (else
          (return false)))
      (else
        (return false)))
    (else
      (return false))))

(fn RestartRound
  (bind _returnvalue (Game|GetPlayerController 0))
  (if (Variables|Default|GetbVictory)
    (Input|ResetIgnoreMoveInput _returnvalue)
    (Input|ResetIgnoreLookInput _returnvalue)
    (Game|SetGamePaused false)
    (bind _returnvalue_2 (Game|GetCurrentLevelName true))
    (Game|OpenLevel(byName) (Utilities|String|StringToName _returnvalue_2))
    (return)
    (else
      (return))))

(fn ShowVictory
  (bind _returnvalue (Game|GetPlayerController 0))
  (bind _returnvalue_2 (Game|GetPlayerCameraManager 0))
  (bind _returnvalue_3 (Math|Vector|MakeVector 1.2e+02 1.2e+02 1.2e+02))
  (bind _victorypanel (Variables|Default|GetVictoryPanel))
  (bind _returnvalue_4 (Camera|GetCameraLocation _returnvalue_2))
  (bind _returnvalue_5 (Camera|GetCameraRotation _returnvalue_2))
  (bind _returnvalue_6 (Math|Vector|GetForwardVector _returnvalue_5))
  (bind _returnvalue_7 (* _returnvalue_6 _returnvalue_3))
  (bind _returnvalue_8 (+ _returnvalue_4 _returnvalue_7))
  (if (Class|HeadMountedDisplayFunctionLibrary|IsHeadMountedDisplayEnabled)
    (Transformation|SetWorldLocation _victorypanel _returnvalue_8 false true)
    (Transformation|SetWorldRotation _victorypanel (Math|Rotator|FindLookatRotation _returnvalue_8 _returnvalue_4) false true)
    (Rendering|SetVisibility _victorypanel true false)
    (Collision|SetCollisionProfileName _victorypanel "UI" true :!class /Script/Engine.PrimitiveComponent)
    (Collision|SetCollisionEnabled _victorypanel "QueryOnly")
    (Variables|Default|SetVictoryWidget (UserInterface|GetUserWidgetObject _victorypanel))
    (bind _aswbp_collection_victory (Utilities|Casting|CastToWBP_CollectionVictory (Variables|Default|GetVictoryWidget)))
    (Default|SetResultCounts _aswbp_collection_victory (Variables|Default|GetStoredLizards) (Variables|Default|GetTotalLizards))
    (return)
    (else
      (bind _returnvalue_9 (Class|WidgetBlueprintLibrary|Create "/Game/CatchTheLizard/WBP_CollectionVictory.WBP_CollectionVictory_C" _returnvalue))
      (Variables|Default|SetVictoryWidget _returnvalue_9)
      (UserInterface|Viewport|AddtoViewport (Variables|Default|GetVictoryWidget) 100)
      (bind _aswbp_collection_victory_2 (Utilities|Casting|CastToWBP_CollectionVictory (Variables|Default|GetVictoryWidget)))
      (Default|SetResultCounts _aswbp_collection_victory_2 (Variables|Default|GetStoredLizards) (Variables|Default|GetTotalLizards))
      (Variables|/Script/Engine.PlayerController|SetbShowMouseCursor _returnvalue true)
      (Input|SetInputModeGameandUI _returnvalue (Variables|Default|GetVictoryWidget) "DoNotLock" false false)
      (return))))

(fn UpdateVictoryInput
  (if (Variables|Default|GetbVictory)
    (if (Variables|Default|GetbVictoryUIArmed)
      (CallFunction|UpdateVictoryLeft)
      (CallFunction|UpdateVictoryRight)
      (return)
      (elif (and (< (Variables|Default|GetLeftTriggerValue) 0.2) (< (Variables|Default|GetRightTriggerValue) 0.2))
        (Variables|Default|SetbVictoryUIArmed true)
        (return)
        (else
          (return))))
    (else
      (return))))

(fn UpdateVictoryLeft
  (if (>= (Variables|Default|GetLeftTriggerValue) 0.5)
    (if (not (Variables|Default|GetbUILeftPressed))
      (Variables|Default|SetbUILeftPressed true)
      (Class|WidgetInteractionComponent|PressPointerKey (Variables|/Game/XRFramework/Blueprints/BP_XRPawn.BP_XRPawn_C|GetWidgetInteractionLeft (Variables|Default|GetPlayerPawnRef)) "(")
      (return)
      (else
        (return)))
    (elif (Variables|Default|GetbUILeftPressed)
      (Variables|Default|SetbUILeftPressed false)
      (Class|WidgetInteractionComponent|ReleasePointerKey (Variables|/Game/XRFramework/Blueprints/BP_XRPawn.BP_XRPawn_C|GetWidgetInteractionLeft (Variables|Default|GetPlayerPawnRef)) "(")
      (return)
      (else
        (return)))))

(fn UpdateVictoryRight
  (if (>= (Variables|Default|GetRightTriggerValue) 0.5)
    (if (not (Variables|Default|GetbUIRightPressed))
      (Variables|Default|SetbUIRightPressed true)
      (Class|WidgetInteractionComponent|PressPointerKey (Variables|/Game/XRFramework/Blueprints/BP_XRPawn.BP_XRPawn_C|GetWidgetInteractionRight (Variables|Default|GetPlayerPawnRef)) "(")
      (return)
      (else
        (return)))
    (elif (Variables|Default|GetbUIRightPressed)
      (Variables|Default|SetbUIRightPressed false)
      (Class|WidgetInteractionComponent|ReleasePointerKey (Variables|/Game/XRFramework/Blueprints/BP_XRPawn.BP_XRPawn_C|GetWidgetInteractionRight (Variables|Default|GetPlayerPawnRef)) "(")
      (return)
      (else
        (return)))))